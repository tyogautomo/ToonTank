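; BP_PawnTank is a tank pawn Blueprint whose only active logic adjusts the sign of its turn speed.
; Every tick it reads MoveForward and keeps TurnSpeed negative at exactly -1, full reverse, and positive otherwise, so steering inverts when backing up.
; The file contains no movement or turning code that consumes TurnSpeed, and its construction script is empty.
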(event `self.ReceiveTick`
  (params (DeltaSeconds :type "Float (single-precision)"))
  (bind _turnspeed (`self.TurnSpeed`))
  (if (== (`self.GetInputAxisValue`) -1.0)
    (if (< _turnspeed 0.0)
      (set `self.TurnSpeed` (* _turnspeed 1.0))
      (else
        (set `self.TurnSpeed` (* _turnspeed -1.0))))
    (else
      (set `self.TurnSpeed` (`KismetMathLibrary.Abs` _turnspeed)))))

(fn `UserConstructionScript`)